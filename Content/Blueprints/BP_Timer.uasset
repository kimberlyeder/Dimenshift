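; BP_Timer is a countdown timer that sends the player's BP_CAVECharacter back to start again when time runs out.
; While StartTimer is true, Tick subtracts delta seconds from TimerValue, shows it on TextTimer and prints it.
; At zero or below, it teleports the character to the first actor tagged "Level2".
; This file never resets TimerValue or StartTimer, so the teleport repeats each tick while the flag stays true.
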(event `self.ReceiveTick`
  (params (DeltaSeconds :type "Float (single-precision)"))
  (if (`self.bStartTimer`)
    (bind _output_get (set `self.TimerValue` (- (`self.TimerValue`) DeltaSeconds)))
    (bind _returnvalue (`KismetTextLibrary.Conv_DoubleToText` _output_get "HalfToEven" false true 2 324 0 0))
    (`KismetSystemLibrary.PrintString` (`KismetTextLibrary.Conv_TextToString` _returnvalue))
    (`TextRenderComponent.K2_SetText` (`self.Text_Timer`) _returnvalue)
    ;[1 1 1] If time = 0, player has to start again
    (if (<= (`self.TimerValue`) 0.0)
      (bind _asbp_cavecharacter (cast `/Game/Blueprints/BP_CAVECharacter` (`GameplayStatics.GetPlayerCharacter` 0)))
      (bind _outactors (`GameplayStatics.GetAllActorsOfClassWithTag` "/Script/Engine.Actor" "Level2"))
      (`self.K2_TeleportTo` :`self` _asbp_cavecharacter :`DestLocation` (`self.K2_GetActorLocation` (`|GetArrayItem` _outactors)))
      (`KismetSystemLibrary.PrintString` "TELEPORT!"))))

(fn `UserConstructionScript`)